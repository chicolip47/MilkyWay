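; BP_Artemis is the top-down player character, with movement, interaction and quest persistence.
; A per-tick camera trace tracks the looked-at interactable for Interact, while IA_Interact uses sphere overlaps to advance NPC dialogue or trigger interactables.
; Non-NPC interaction results are broadcast as quest objective IDs.
; Quests load from the GameInstance's save data on BeginPlay, and a debug-style key 2 press writes them to the save slot.
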(event `self.ReceiveBeginPlay`
  (bind _asplayer_controller (cast `PlayerController` (`self.GetController`)))
  (`EnhancedInputSubsystemInterface.AddMappingContext` (pcsubsystem `EnhancedInputLocalPlayerSubsystem` _asplayer_controller) "/Game/Input_Character/IMC_TopDown.IMC_TopDown" 0 (struct))
  (bind _asmy_game_instance (cast `/Game/SavingSystem/MyGameInstance` (`GameplayStatics.GetGameInstance`)))
  (bind _output_get (set `self.As My Game Instance` _asmy_game_instance))
  (`/Game/SavingSystem/MySaveData.LoadQuests` (`/Game/SavingSystem/MyGameInstance.SaveData` _output_get) (`self.QuestLogComponent`)))

(event `EnhancedInput|/Game/Input_Character/Actions/IA_Move`
  (params (ActionValue :type "Vector2D Structure") (ElapsedSeconds :type "Float (double-precision)") (TriggeredSeconds :type "Float (double-precision)") (InputAction :type "InputAction Object Reference" :default "/Game/Input_Character/Actions/IA_Move.IA_Move"))
  (bind (_x _y) (`KismetMathLibrary.BreakVector2D` ActionValue))
  ; Movimento
  (:`Triggered`
    (`self.AddMovementInput` (1.0 0.0 0.0) _x)
    (`self.AddMovementInput` (0.0 1.0 0.0) _y)))

(event `self.ReceiveTick`
  (params (DeltaSeconds :type "Float (single-precision)"))
  (`self.InteractTrace`))

(event `InputAction|Interact`
  (params (Key :type "Key Structure"))
  (:`Pressed`
    (bind _lookatactor (`self.LookAtActor`)
      (:`then`
        (bind _objectiveid (message `/Game/I_InteractionInterface.InteractWith` _lookatactor))
        (`self.OnObjectiveIDCalled` _objectiveid))
      (:`else`))))

(event `EnhancedInput|/Game/Input_Character/Actions/IA_Interact`
  (params (ActionValue :type Boolean) (ElapsedSeconds :type "Float (double-precision)") (TriggeredSeconds :type "Float (double-precision)") (InputAction :type "InputAction Object Reference" :default "/Game/Input_Character/Actions/IA_Interact.IA_Interact"))
  (:`Triggered`
    (for _array_element (`PrimitiveComponent.GetOverlappingActors` (`self.Sphere`) "/Game/Blueprints/BP_Interactable.BP_Interactable_C")
      (bind _asbp_npc (cast `/Game/Blueprints/BP_NPC` _array_element)
        (:`then`
          (if (`/Game/Blueprints/BP_NPC.isFirstInteraction?` _asbp_npc)
            (set `/Game/Blueprints/BP_NPC.isFirstInteraction?` false _asbp_npc))
          (message `/Game/I_InteractionInterface.Talk` _asbp_npc)
          (`/Game/Blueprints/BP_NPC.incrementTextIndex` _asbp_npc))
        (:`CastFailed`
          (bind _asbp_interactable (cast `/Game/Blueprints/BP_Interactable` _array_element))
          (bind _objectiveid (message `/Game/I_InteractionInterface.InteractWith` _asbp_interactable))
          (`self.OnObjectiveIDCalled` _objectiveid 1))))))

(event `Key|Two`
  (params (Key :type "Key Structure"))
  (bind _savedata (`/Game/SavingSystem/MyGameInstance.SaveData` (`self.As My Game Instance`)))
  (:`Pressed`
    (bind _asmy_game_instance (cast `/Game/SavingSystem/MyGameInstance` (`GameplayStatics.GetGameInstance`)))
    (set `self.As My Game Instance` _asmy_game_instance)
    (for _array_element (`/Game/QuestSystem/QuestLogComponent.CurrentQuests` (`self.QuestLogComponent`))
      (`/Game/SavingSystem/MySaveData.SaveQuestDetails` _savedata _array_element))
    (`/Game/SavingSystem/MySaveData.SaveQuestLog` _savedata (`self.QuestLogComponent`))
    (`GameplayStatics.SaveGameToSlot` (`/Game/SavingSystem/MyGameInstance.SaveData` (`self.As My Game Instance`)) "savedata")))

(fn `InteractTrace`
  (bind _returnvalue (`GameplayStatics.GetPlayerCameraManager` 0))
  (bind _returnvalue_2 (`self.K2_GetActorLocation` _returnvalue))
  ; Interact Trace
  (bind (_outhit _returnvalue_3) (`KismetSystemLibrary.LineTraceSingle` _returnvalue_2 (+ _returnvalue_2 (* (`self.GetActorForwardVector` _returnvalue) 200.0)) "TraceTypeQuery2"))
  (if _returnvalue_3
    (bind (_bblockinghit _binitialoverlap _time _distance _location _impactpoint _normal _impactnormal _physmat _hitactor) (`GameplayStatics.BreakHitResult` _outhit))
    (if (`KismetSystemLibrary.DoesImplementInterface` _hitactor)
      (bind _output_get (set `self.LookAtActor` _hitactor))
      (message `/Game/I_InteractionInterface.LookAt` _output_get)
      (else
        (set `self.LookAtActor` null)))
    (else
      (set `self.LookAtActor` null))))

(fn `InteractWith`
  (returns (ObjectiveID :type String))
  (return ""))

(fn `LookAt`
  (returns (InteractText :type Text))
  (return ""))

(fn `UserConstructionScript`)