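; BP_NPC is an NPC that serves dialogue lines and a portrait from a DialogueAsset.
; Talk selects the first node matching the current QuestState and Stage, then returns the line at the index saved for that quest state.
; IncrementTextIndex advances that per-state index, resetting it and hiding dialogue on the BP_Artemis player pawn once past the end.
; InteractWith and LookAt return empty strings.
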(fn `getSpeakerName`
  (returns (Speaker :type Name))
  (bind _dialogueasset (`self.DialogueAsset`)
    (:`then`
      (return (`/Game/DialogueSystem/DA_DialogueBase.SpeakerName` _dialogueasset)))
    (:`else`)))

(fn `incrementTextIndex`
  (bind (_value _returnvalue) (`BlueprintMapLibrary.Map_Find` (`self.LastDialogueIndex`) (`self.QuestState`)))
  (if _returnvalue
    (if (<= _value (- (`KismetArrayLibrary.Array_Length` (`.DialogueText_15_C30F0AFA41C56FC0E26C76A1146ADEF8` (break `/Game/DialogueSystem/F_DialogueNode` (`self.currentDialogueNode`)))) 1))
      (`BlueprintMapLibrary.Map_Add` (`self.LastDialogueIndex`) (`self.QuestState`) (+ _value 1))
      (else
        (`BlueprintMapLibrary.Map_Add` (`self.LastDialogueIndex`) (`self.QuestState`))
        (bind _asbp_artemis (cast `/Game/Blueprints/Artemis/BP_Artemis` (`GameplayStatics.GetPlayerPawn` 0)))
        (`/Game/Blueprints/Artemis/BP_Artemis.HideDialogue` _asbp_artemis)))))

(fn `InteractWith`
  (returns (ObjectiveID :type String))
  (return ""))

(fn `LookAt`
  (returns (InteractText :type Text))
  (return ""))

(fn `matchingDialogueNode`
  (params (analyzedNode :type "/Game/DialogueSystem/F_DialogueNode Structure"))
  (returns (dialogueNode :type "/Game/DialogueSystem/F_DialogueNode Structure") (`isMatching?` :type Boolean))
  (bind (_id _npcqueststate _stage) (break `/Game/DialogueSystem/F_DialogueNode` analyzedNode))
  (if (and (`|EnumEquality` _npcqueststate (`self.QuestState`)) (== (`self.Stage`) _stage))
    (return analyzedNode true)
    (else
      (return (struct) false))))

(fn `Talk`
  (returns (dialogue :type Text) (portrait :type "Texture2D Object Reference") (speaker :type Text))
  (bind (_currentdialoguenode_id _currentdialoguenode_npcqueststate _currentdialoguenode_stage _currentdialoguenode_speakername _currentdialoguenode_dialoguetext) (break `/Game/DialogueSystem/F_DialogueNode` (`self.currentDialogueNode`)))
  (bind (_value _returnvalue) (`BlueprintMapLibrary.Map_Find` (`self.LastDialogueIndex`) (`self.QuestState`)))
  (bind _dialogueasset (`self.DialogueAsset`)
    (:`then`
      (for _array_element (`/Game/DialogueSystem/DA_DialogueBase.Nodes` _dialogueasset)
        (bind (_dialoguenode _ismatching_) (`self.matchingDialogueNode` _array_element))
        (if _ismatching_
          (set `self.currentDialogueNode` _dialoguenode)
          (break)))
      (if (> (`KismetArrayLibrary.Array_Length` _currentdialoguenode_dialoguetext) 0)
        (if _returnvalue
          (return (`|GetArrayItem` _currentdialoguenode_dialoguetext _value) (`self.portrait`) _currentdialoguenode_speakername))))
    (:`else`)))

(fn `UserConstructionScript`)