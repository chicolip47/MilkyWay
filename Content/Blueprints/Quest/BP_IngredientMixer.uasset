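; Interactable ingredient mixer that holds up to three ingredients and checks them against recipes.
; CombineIngredients scans RecipesDataTable, matching ingredient types against two- or three-ingredient recipes through temporary found flags, and returns the recipe name and icon.
; ObjectInteracted runs the combine and prints the result, with a debug print standing in for the planned mix widget.
; InteractWith, LookAt and Talk are empty stubs.
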(event `/Game/I_InteractionInterface.ObjectInteracted`
  (params (Interactor :type "Actor Object Reference"))
  (`KismetSystemLibrary.PrintString` "CREATE AND ACTIVATE MIX WIDGET GLI PASSO ANCHE LA REFERENCE DI QUESTO OGGETTO BP E INVENTORY COMP DEL PLAYER")
  (bind (_combined _recipename) (`self.combineIngredients`))
  (if _combined
    (`KismetSystemLibrary.PrintString` (`KismetTextLibrary.Conv_TextToString` _recipename) true true (struct :`G` 0.66 :`B` 1.0 :`A` 1.0) 22.0)))

(fn `addIngredientToMix`
  (params (item :type "/Game/itemData/F_IngredientAmount Structure"))
  (returns (slot :type Integer))
  (bind _returnvalue (`KismetArrayLibrary.Array_Length` (`self.IngredientsToMix`)))
  (if (== _returnvalue 0)
    (`KismetArrayLibrary.Array_Add` (`self.IngredientsToMix`) item)
    (return 1)
    (elif (== _returnvalue 1)
      (`KismetArrayLibrary.Array_Add` (`self.IngredientsToMix`) item)
      (return 2)
      (elif (== _returnvalue 2)
        (`KismetArrayLibrary.Array_Add` (`self.IngredientsToMix`) item)
        (return 3)))))

(fn `clearIngredients`
  (`KismetArrayLibrary.Array_Clear` (`self.IngredientsToMix`)))

(fn `combineIngredients`
  (returns (combined :type Boolean) (recipeName :type Text) (RecipeIcon :type "Texture2D Object Reference"))
  (locals (tmp1Found :type Boolean) (tmp2Found :type Boolean) (tmp3Found :type Boolean))
  (bind _ingredientstomix (`self.IngredientsToMix`))
  (bind _output_ingredienttype (break `/Game/itemData/F_IngredientAmount` (`|GetArrayItem` _ingredientstomix)))
  (bind _output_ingredienttype_2 (break `/Game/itemData/F_IngredientAmount` (`|GetArrayItem` (`self.IngredientsToMix`) 1)))
  (bind _output_ingredienttype_3 (break `/Game/itemData/F_IngredientAmount` (`|GetArrayItem` (`self.IngredientsToMix`))))
  (bind _output_ingredienttype_4 (break `/Game/itemData/F_IngredientAmount` (`|GetArrayItem` (`self.IngredientsToMix`) 1)))
  (bind _output_ingredienttype_5 (break `/Game/itemData/F_IngredientAmount` (`|GetArrayItem` (`self.IngredientsToMix`))))
  (bind _output_ingredienttype_6 (break `/Game/itemData/F_IngredientAmount` (`|GetArrayItem` (`self.IngredientsToMix`) 2)))
  (if (and (== (`KismetArrayLibrary.Array_Length` _ingredientstomix) 1) (`|EnumEquality` _output_ingredienttype "NewEnumerator0"))
    _
    (elif (or (== (`KismetArrayLibrary.Array_Length` (`self.IngredientsToMix`)) 2) (== (`KismetArrayLibrary.Array_Length` (`self.IngredientsToMix`)) 3))
      (bind _outrownames (`DataTableFunctionLibrary.GetDataTableRowNames` (`self.RecipesDataTable`)))
      (for _array_element _outrownames
        (bind _returnvalue (`|GetDataTableRow` (`self.RecipesDataTable`) _array_element)
          (:`then`
            (bind (_recipetype _displayname _requiredingredients _basevalue _icon) (break `/Game/itemData/F_Recipes` _returnvalue))
            (if (== (`KismetArrayLibrary.Array_Length` _requiredingredients) 2)
              (for _array_element_2 _requiredingredients
                (if (`local.tmp1Found`)
                  (bind _ingredienttype (break `/Game/itemData/F_IngredientAmount` _array_element_2))
                  (if (`|EnumEquality` _output_ingredienttype_4 _ingredienttype) :!label _label
                    (set `local.tmp2Found` true)
                    (else
                      (break)))
                  (elif (`|EnumEquality` _output_ingredienttype_5 _ingredienttype)
                    (set `local.tmp1Found` true)
                    (else
                      (goto _label)))))
              (if (and (`local.tmp1Found`) (`local.tmp2Found`))
                (set `local.tmp2Found` false)
                (set `local.tmp1Found` false)
                (`KismetSystemLibrary.PrintString` "FOUND")
                (return true _displayname _icon)
                (else
                  (set `local.tmp2Found` false)
                  (set `local.tmp1Found` false)))
              (elif (== (`KismetArrayLibrary.Array_Length` _requiredingredients) 3)
                (for _array_element_3 _requiredingredients
                  (if (`local.tmp1Found`)
                    (if (`local.tmp2Found`) :!label _label_2
                      (bind _ingredienttype_2 (break `/Game/itemData/F_IngredientAmount` _array_element_3))
                      (if (`|EnumEquality` _output_ingredienttype_6 _ingredienttype_2) :!label _label_3
                        (set `local.tmp3Found` true)
                        (else
                          (break)))
                      (elif (`|EnumEquality` _output_ingredienttype_2 _ingredienttype_2)
                        (set `local.tmp2Found` true)
                        (else
                          (goto _label_3))))
                    (elif (`|EnumEquality` _output_ingredienttype_3 _ingredienttype_2)
                      (set `local.tmp1Found` true)
                      (else
                        (goto _label_2)))))
                (if (and (`local.tmp1Found`) (`local.tmp2Found`) (`local.tmp3Found`))
                  (set `local.tmp1Found` false)
                  (set `local.tmp2Found` false)
                  (set `local.tmp3Found` false)
                  (`KismetSystemLibrary.PrintString` "FOUND")
                  (return true _displayname _icon)
                  (else
                    (set `local.tmp1Found` false)
                    (set `local.tmp2Found` false)
                    (set `local.tmp3Found` false))))))))
      (return false "" null))))

(fn `InteractWith`
  (returns (ObjectiveID :type String))
  (return ""))

(fn `LookAt`
  (returns (InteractText :type Text))
  (return ""))

(fn `Talk`
  (returns (dialogue :type Text) (portrait :type "Texture2D Object Reference") (speaker :type Text))
  (return "" null ""))

(fn `UserConstructionScript`)