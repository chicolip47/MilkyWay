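; BPC_Dialogue is a dialogue component that lets its owner open a conversation display when interacted with.
; Interaction stores the interactor and creates the dialogue widget with Name and Portrait, or signals speaker finished on the existing widget's dialogue box.
; If the owner has a BP_AIController, it enters a conversing state toward the interactor.
; Ending dialogue removes the widget and returns the AI to idle.
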(event `self.ReceiveBeginPlay`
  ; Set Reference to AI Controller
  (bind _asbp_aicontroller (cast `/Game/AI/BP_AIController` (`AIBlueprintHelperLibrary.GetAIController` (`self.GetOwner`))))
  (set `self.AIController` _asbp_aicontroller))

(event `CreateDialogueDisplay`
  ; Create Dialogue Display
  (`self.DialogueDisplay`
    (:`then`
      (`/Game/DialogueSystem/DialogueUI/W_DialogueBox.OnSpeakerFinished` (`/Game/DialogueSystem/DialogueUI/W_DialogueDisplay.DialogueBox` (`self.DialogueDisplay`))))
    (:`else`
      (bind _returnvalue (`|CreateWidget` "/Game/DialogueSystem/DialogueUI/W_DialogueDisplay.W_DialogueDisplay_C" null (`self.Name`) (`self.Portrait`)))
      (bind _output_get (set `self.DialogueDisplay` _returnvalue))
      (`UserWidget.AddToViewport` _output_get 0)
      (bind _aicontroller (`self.AIController`)
        (:`then`
          (`/Game/AI/BP_AIController.SetStateAsConversating` _aicontroller (`self.Interactor`)))
        (:`else`)))))

(event `/Game/I_InteractionInterface.ObjectInteracted`
  (params (Interactor :type "Actor Object Reference"))
  (set `self.Interactor` Interactor)
  (`self.CreateDialogueDisplay`))

(event `EndDialogue`
  ; End Dialogue Logic
  (bind _dialoguedisplay (`self.DialogueDisplay`)
    (:`then`
      (`Widget.RemoveFromParent` _dialoguedisplay)
      (set `self.DialogueDisplay` null)
      (bind _aicontroller (`self.AIController`)
        (:`then`
          (`/Game/AI/BP_AIController.SetStateAsIdle` _aicontroller))
        (:`else`)))
    (:`else`)))

(fn `InteractWith`
  (returns (ObjectiveID :type String))
  (return ""))

(fn `LookAt`
  (returns (InteractText :type Text))
  (return ""))

(fn `Talk`
  (returns (dialogue :type Text))
  (return ""))