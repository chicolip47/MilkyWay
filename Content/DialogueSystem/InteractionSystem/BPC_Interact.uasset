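; Actor component that lets its owner detect nearby interactable objects and interact with them through I_InteractionInterface.
; On BeginPlay it adds a W_Interact widget to the viewport.
; Each Tick, a zero-length sphere trace at the owner's location stores an interface-implementing hit as HitTarget and shows its look-at message, otherwise clearing both.
; The IA_Interact input sends ObjectInteractedMessage to a valid HitTarget, passing the owner.
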(event `self.ReceiveBeginPlay`
  (`self.CreateInteractDisplay`))

(event `self.ReceiveTick`
  (params (DeltaSeconds :type "Float (single-precision)"))
  (`self.InteractionTrace`))

(event `CreateInteractDisplay`
  ; Create Interaction Display
  (bind _returnvalue (`|CreateWidget` "/Game/DialogueSystem/UI/W_Interact.W_Interact_C"))
  (bind _output_get (set `self.InteractDisplay` _returnvalue))
  (`UserWidget.AddToViewport` _output_get 0))

(event `EnhancedInput|/Game/Input_Character/Actions/IA_Interact`
  (params (ActionValue :type Boolean) (ElapsedSeconds :type "Float (double-precision)") (TriggeredSeconds :type "Float (double-precision)") (InputAction :type "InputAction Object Reference" :default "/Game/Input_Character/Actions/IA_Interact.IA_Interact"))
  ; Interaction input
  (:`Started`
    (bind _hittarget (`self.HitTarget`)
      (:`then`
        (message `/Game/I_InteractionInterface.ObjectInteracted` _hittarget (`self.GetOwner`)))
      (:`else`))))

(fn `InteractionTrace`
  (bind _returnvalue (`Actor.K2_GetActorLocation` (`self.GetOwner`)))
  (bind (_outhit _returnvalue_2) (`KismetSystemLibrary.SphereTraceSingle` _returnvalue _returnvalue (`self.InteractRadius`) "TraceTypeQuery3"))
  (if _returnvalue_2
    (bind (_bblockinghit _binitialoverlap _time _distance _location _impactpoint _normal _impactnormal _physmat _hitactor) (`GameplayStatics.BreakHitResult` _outhit))
    (if (`KismetSystemLibrary.DoesImplementInterface` _hitactor "/Game/I_InteractionInterface.I_InteractionInterface_C")
      (bind _output_get (set `self.HitTarget` _hitactor))
      (bind _interacttext (message `/Game/I_InteractionInterface.LookAt` _output_get))
      (`/Game/DialogueSystem/UI/W_Interact.UpdateInteractText` (`self.InteractDisplay`) _interacttext)
      (else
        (set `self.HitTarget` null)
        (`/Game/DialogueSystem/UI/W_Interact.UpdateInteractText` (`self.InteractDisplay`) "")))
    (else
      (set `self.HitTarget` null)
      (`/Game/DialogueSystem/UI/W_Interact.UpdateInteractText` (`self.InteractDisplay`) ""))))