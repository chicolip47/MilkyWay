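; BP_GasStation is a fuel pump trigger that tells overlapping actors they are at the pump and shows the fill-gas UI.
; Sphere begin overlap sends InThePumpMessage(true) and creates the W_FillGas widget, with a DoOnce preventing duplicates.
; End overlap sends false, removes the widget and resets the DoOnce, with no filtering by actor type.
; Its own InThePump function is a stub returning false.
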(event `self.Sphere.OnComponentBeginOverlap`
  (params (OverlappedComponent :type "PrimitiveComponent Object Reference") (OtherActor :type "Actor Object Reference") (OtherComp :type "PrimitiveComponent Object Reference") (OtherBodyIndex :type Integer) (bFromSweep :type Boolean) (SweepResult :type "HitResult Structure (by ref)"))
  (message `/Game/GameManager_SpaceShip/BPI_SpaceShip.InThePump` OtherActor true)
  (`/Engine/EditorBlueprintResources/StandardMacros.DoOnce` false :!label _label
    (:`Completed`
      (bind _returnvalue (`|CreateWidget` "/Game/FuelSystem/W_FillGas.W_FillGas_C"))
      (bind _output_get (set `self.UMGPetrol` _returnvalue))
      (`UserWidget.AddToViewport` _output_get 0))))

(event `self.Sphere.OnComponentEndOverlap`
  (params (OverlappedComponent :type "PrimitiveComponent Object Reference") (OtherActor :type "Actor Object Reference") (OtherComp :type "PrimitiveComponent Object Reference") (OtherBodyIndex :type Integer))
  (message `/Game/GameManager_SpaceShip/BPI_SpaceShip.InThePump` OtherActor false)
  (`Widget.RemoveFromParent` (`self.UMGPetrol`))
  (goto _label :!via `Reset`))

(fn `InThePump`
  (params (InPump :type Boolean))
  (returns (OutPump :type Boolean))
  (return false))

(fn `UserConstructionScript`)