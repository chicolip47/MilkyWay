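; Player controller for the spaceship mode that adds the spaceship input mapping, shows the gas bar on start and opens a quest log on Tab.
; Enhanced Input look, roll and thrust actions go to the controlled pawn as messages, with thrust start and release toggling deceleration.
; Thrust also sets the moving flag on the cached BP_SpaceShip.
; Refuel input calls RefillFuel only when the cached BP_Benzinaio reports the player nearby.
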(event `Key|Tab`
  (params (Key :type "Key Structure"))
  (:`Pressed`
    (bind _returnvalue (`|CreateWidget` "/Game/QuestSystem/UI/W_QuestLog.W_QuestLog_C"))
    (`UserWidget.AddToViewport` _returnvalue 0)))

(event `self.ReceiveBeginPlay`
  (`EnhancedInputSubsystemInterface.AddMappingContext` (subsystem `EnhancedInputLocalPlayerSubsystem`) "/Game/GameManager_SpaceShip/Input_SpaceShip/IMC_Spaceship.IMC_Spaceship" 0 (struct))
  (bind _returnvalue (`|CreateWidget` "/Game/FuelSystem/W_GasBar.W_GasBar_C"))
  (`UserWidget.AddToViewport` _returnvalue 0)
  (bind _returnvalue_2 (`GameplayStatics.GetActorOfClass` "/Game/SpaceShip/BP_SpaceShip.BP_SpaceShip_C"))
  (set `self.As BP Space Ship` _returnvalue_2)
  (bind _returnvalue_3 (`GameplayStatics.GetActorOfClass` "/Game/FuelSystem/BP_Benzinaio.BP_Benzinaio_C"))
  (set `self.Benzinaio` _returnvalue_3))

(event `EnhancedInput|/Game/GameManager_SpaceShip/Input_SpaceShip/IA_LookLeftRight`
  (params (ActionValue :type "Float (double-precision)") (ElapsedSeconds :type "Float (double-precision)") (TriggeredSeconds :type "Float (double-precision)") (InputAction :type "InputAction Object Reference" :default "/Game/GameManager_SpaceShip/Input_SpaceShip/IA_LookLeftRight.IA_LookLeftRight"))
  (:`Triggered`
    (message `/Game/GameManager_SpaceShip/BPI_SpaceShip.Look Right & Left` (`self.K2_GetPawn`) ActionValue)))

(event `EnhancedInput|/Game/GameManager_SpaceShip/Input_SpaceShip/IA_LookUpDown`
  (params (ActionValue :type "Float (double-precision)") (ElapsedSeconds :type "Float (double-precision)") (TriggeredSeconds :type "Float (double-precision)") (InputAction :type "InputAction Object Reference" :default "/Game/GameManager_SpaceShip/Input_SpaceShip/IA_LookUpDown.IA_LookUpDown"))
  (:`Triggered`
    (message `/Game/GameManager_SpaceShip/BPI_SpaceShip.Look Top & Down` (`self.K2_GetPawn`) ActionValue)))

(event `EnhancedInput|/Game/GameManager_SpaceShip/Input_SpaceShip/IA_Roll`
  (params (ActionValue :type "Float (double-precision)") (ElapsedSeconds :type "Float (double-precision)") (TriggeredSeconds :type "Float (double-precision)") (InputAction :type "InputAction Object Reference" :default "/Game/GameManager_SpaceShip/Input_SpaceShip/IA_Roll.IA_Roll"))
  (:`Triggered`
    (message `/Game/GameManager_SpaceShip/BPI_SpaceShip.Roll Right & Left` (`self.K2_GetPawn`) ActionValue)))

(event `EnhancedInput|/Game/GameManager_SpaceShip/Input_SpaceShip/IA_MoveSpaceShip`
  (params (ActionValue :type "Float (double-precision)") (ElapsedSeconds :type "Float (double-precision)") (TriggeredSeconds :type "Float (double-precision)") (InputAction :type "InputAction Object Reference" :default "/Game/GameManager_SpaceShip/Input_SpaceShip/IA_MoveSpaceShip.IA_MoveSpaceShip"))
  (bind _returnvalue (`self.K2_GetPawn`))
  (:`Triggered`
    (message `/Game/GameManager_SpaceShip/BPI_SpaceShip.Move SpaceShip` _returnvalue (> ActionValue 0.0))
    (set `/Game/SpaceShip/BP_SpaceShip.bIsMoving?` true (`self.As BP Space Ship`)))
  (:`Started`
    (message `/Game/GameManager_SpaceShip/BPI_SpaceShip.Start Deceleration` _returnvalue false))
  (:`Completed`
    (message `/Game/GameManager_SpaceShip/BPI_SpaceShip.Start Deceleration` _returnvalue true)
    (set `/Game/SpaceShip/BP_SpaceShip.bIsMoving?` false (`self.As BP Space Ship`))))

(event `EnhancedInput|/Game/GameManager_SpaceShip/Input_SpaceShip/IA_RefillGas`
  (params (ActionValue :type "Float (double-precision)") (ElapsedSeconds :type "Float (double-precision)") (TriggeredSeconds :type "Float (double-precision)") (InputAction :type "InputAction Object Reference" :default "/Game/GameManager_SpaceShip/Input_SpaceShip/IA_RefillGas.IA_RefillGas"))
  (:`Triggered`
    (bind _benzinaio (`self.Benzinaio`)
      (:`then`
        (if (`/Game/FuelSystem/BP_Benzinaio.bIsPlayerNear?` _benzinaio)
          (bind _asbp_space_ship (cast `/Game/SpaceShip/BP_SpaceShip` (`self.K2_GetPawn`)))
          (`/Game/SpaceShip/BP_SpaceShip.RefillFuel` _asbp_space_ship)))
      (:`else`))))

(fn `UserConstructionScript`)