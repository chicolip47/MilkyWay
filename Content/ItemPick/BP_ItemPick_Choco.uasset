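; BP_ItemPick_Choco is an interactable ingredient pickup, named for chocolate, that supplies the player's inventory.
; When interacted with, it casts the interactor to BP_Artemis, stores that reference, and adds its configured ingredient type and quantity to that character's InventoryComponent.
; The actor neither destroys nor disables itself afterward.
; Its InteractWith, LookAt and Talk functions return empty text, and its other events do nothing.
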(event `/Game/I_InteractionInterface.ObjectInteracted`
  (params (Interactor :type "Actor Object Reference"))
  (bind _asbp_artemis (cast `/Game/Blueprints/Artemis/BP_Artemis` Interactor))
  (bind _output_get (set `self.PlayerReference` _asbp_artemis))
  (`/Game/QuestSystem/InventoryComponent.AddToInventory` (`/Game/Blueprints/Artemis/BP_Artemis.InventoryComponent` _output_get) (`self.QuantitaFornita`) (`self.TipoDiIngrediente`)))

(fn `InteractWith`
  (returns (ObjectiveID :type String))
  (return ""))

(fn `LookAt`
  (returns (InteractText :type Text))
  (return ""))

(fn `Talk`
  (returns (dialogue :type Text) (portrait :type "Texture2D Object Reference") (speaker :type Text))
  (return "" null ""))

(fn `UserConstructionScript`)