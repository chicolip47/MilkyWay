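; BP_CEO is an interactable CEO character that the player can talk to through a dialogue component.
; Interaction events pass the interactor to BPCDialogue, and any end of overlap with InteractionRadius ends the dialogue.
; LookAt builds a "Talk to" prompt from the character's Name, while InteractWith and Talk return empty strings.
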(event `/Game/I_InteractionInterface.ObjectInteracted`
  (params (Interactor :type "Actor Object Reference"))
  (`/Game/I_InteractionInterface.ObjectInteracted` (`self.BPC_Dialogue`) Interactor))

(event `self.InteractionRadius.OnComponentEndOverlap`
  (params (OverlappedComponent :type "PrimitiveComponent Object Reference") (OtherActor :type "Actor Object Reference") (OtherComp :type "PrimitiveComponent Object Reference") (OtherBodyIndex :type Integer))
  (`/Game/Dialogue/BPC_Dialogue.EndDialogue` (`self.BPC_Dialogue`)))

(fn `InteractWith`
  (returns (ObjectiveID :type String))
  (return ""))

(fn `LookAt`
  (returns (InteractText :type Text))
  (return (`|FormatText` "Talk to {x}" (`self.Name`))))

(fn `Talk`
  (returns (dialogue :type Text) (portrait :type "Texture2D Object Reference") (speaker :type Text))
  (return "" null ""))

(fn `UserConstructionScript`)