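; BP_Mucca1 is a Terra planet actor that gets pulled toward the player and shrinks away when they come close.
; Its Sphere overlap sets or clears the player as Target and starts or clears a looping timer.
; While Target is valid, Tick applies a delta-time-scaled move along the direction to the player, as a local offset without sweep.
; Each pull also shrinks the mesh by a fixed per-call step, destroying the actor at zero scale.
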(event `self.ReceiveTick`
  (params (DeltaSeconds :type "Float (single-precision)"))
  (`self.Target`
    (:`then`
      (`self.PullTowardsTarget`))
    (:`else`)))

(event `self.Sphere.OnComponentBeginOverlap`
  (params (OverlappedComponent :type "PrimitiveComponent Object Reference") (OtherActor :type "Actor Object Reference") (OtherComp :type "PrimitiveComponent Object Reference") (OtherBodyIndex :type Integer) (bFromSweep :type Boolean) (SweepResult :type "HitResult Structure (by ref)"))
  (if (== OtherActor (`GameplayStatics.GetPlayerCharacter` 0))
    (set `self.Target` OtherActor)
    (bind _returnvalue (`KismetSystemLibrary.K2_SetTimerDelegate` (`|CreateDelegate` :!event `PullTowardsTarget`) 0.0 true))
    (set `self.Timer` _returnvalue)))

(event `self.Sphere.OnComponentEndOverlap`
  (params (OverlappedComponent :type "PrimitiveComponent Object Reference") (OtherActor :type "Actor Object Reference") (OtherComp :type "PrimitiveComponent Object Reference") (OtherBodyIndex :type Integer))
  (if (== OtherActor (`GameplayStatics.GetPlayerCharacter` 0))
    (set `self.Target` null)
    (`KismetSystemLibrary.K2_ClearAndInvalidateTimerHandle` (`self.Timer`))))

(event `PullTowardsTarget`
  (bind _staticmesh (`self.StaticMesh`))
  (bind _relativescale3d_x (`KismetMathLibrary.BreakVector` (`SceneComponent.RelativeScale3D` _staticmesh)))
  (`self.K2_AddActorLocalOffset` (* (`KismetMathLibrary.Normal` (- (`self.K2_GetActorLocation` (`self.Target`)) (`self.K2_GetActorLocation`))) (`GameplayStatics.GetWorldDeltaSeconds`) (`self.Speed`)))
  (`SceneComponent.SetRelativeScale3D` _staticmesh (- (`SceneComponent.RelativeScale3D` _staticmesh) (0.01 0.01 0.01)))
  (if (<= _relativescale3d_x 0.0)
    (`self.K2_DestroyActor`)))

(fn `UserConstructionScript`)